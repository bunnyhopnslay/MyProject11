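; BP_Player is a player character Blueprint with click-to-move control.
; BeginPlay shows the mouse cursor for the first player controller.
; When IA_ClickDestination starts, a Visibility line trace runs from the deprojected cursor position along its direction for Distance, with timed debug drawing.
; On a hit, SimpleMoveToLocation sends the pawn's controller to the hit location through navigation pathfinding.
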(event `self.ReceiveBeginPlay`
  (set `PlayerController.bShowMouseCursor` true (`GameplayStatics.GetPlayerController` 0)))

(event `EnhancedInput|/Game/Input/Actions/IA_ClickDestination`
  (params (ActionValue :type Boolean) (ElapsedSeconds :type "Float (double-precision)") (TriggeredSeconds :type "Float (double-precision)") (InputAction :type "InputAction Object Reference" :default "/Game/Input/Actions/IA_ClickDestination.IA_ClickDestination"))
  (bind (_worldlocation _worlddirection) (`PlayerController.DeprojectMousePositionToWorld` (`GameplayStatics.GetPlayerController` 0)))
  (:`Started`
    (bind (_outhit _returnvalue) (`KismetSystemLibrary.LineTraceSingle` :`Start` _worldlocation :`End` (+ _worldlocation (* _worlddirection (`self.Distance`))) :`TraceChannel` "TraceTypeQuery1" :`DrawDebugType` "ForDuration"))
    (if _returnvalue
      (`AIBlueprintHelperLibrary.SimpleMoveToLocation` (`self.GetController`) (`.Location` (`GameplayStatics.BreakHitResult` _outhit))))))

(fn `UserConstructionScript`)