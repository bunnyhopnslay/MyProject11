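; Player controller for mouse click-to-move control of the pawn, using Enhanced Input.
; BeginPlay adds the default mapping context, and pressing the click action stops current movement.
; While triggered, it caches the visibility trace hit under the cursor and steers the pawn toward it with movement input.
; A release before the press threshold instead calls SimpleMoveToLocation to the cached point and spawns an effect system there.
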(event `self.ReceiveBeginPlay`
  (bind _returnvalue (subsystem `EnhancedInputLocalPlayerSubsystem`))
  ;[0.01718 0.05098 0.01235] Les inputs donner au player
  (`/Engine/EditorBlueprintResources/StandardMacros.IsValid` _returnvalue
    (:`Is Valid`
      (`EnhancedInputSubsystemInterface.AddMappingContext` _returnvalue "/Game/Input/IMC_Default.IMC_Default" 0 (struct)))))

(event `EnhancedInput|/Game/Input/Actions/IA_ClickDestination`
  (params (ActionValue :type Boolean) (ElapsedSeconds :type "Float (double-precision)") (TriggeredSeconds :type "Float (double-precision)") (InputAction :type "InputAction Object Reference" :default "/Game/Input/Actions/IA_ClickDestination.IA_ClickDestination"))
  (bind (_hit _location) (`self.GetLocationUnderCursor`))
  (:`Triggered`
    (if _hit
      (bind _output_get (set `self.CachedDestination` _location))
      (`self.Follow` _output_get)))
  (:`Started`
    (`self.StopMovement`))
  (:`Canceled`
    (if (< ElapsedSeconds (`self.PressedThreshold`)) :!label _label
      (`self.MoveTo` (`self.CachedDestination`))))
  (:`Completed`
    (goto _label)))

(fn `Follow`
  (params (Location :type "Vector Structure"))
  (bind _returnvalue (`self.K2_GetPawn`))
  (`Pawn.AddMovementInput` _returnvalue (`KismetMathLibrary.GetDirectionUnitVector` (`self.K2_GetActorLocation` _returnvalue) Location) 1.0 false))

(fn `GetLocationUnderCursor`
  (returns (Hit :type Boolean) (Location :type "Vector Structure"))
  (bind (_bblockinghit _binitialoverlap _time _distance _location) (`GameplayStatics.BreakHitResult` (`self.GetHitResultUnderCursorByChannel` "TraceTypeQuery1")))
  (return _bblockinghit _location))

(fn `MoveTo`
  (params (Location :type "Vector Structure"))
  (`AIBlueprintHelperLibrary.SimpleMoveToLocation` self Location)
  (`NiagaraFunctionLibrary.SpawnSystemAtLocation` null Location))

(fn `UserConstructionScript`)